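; Rifle weapon Blueprint that adds Chaos physics field impacts where its shots hit.
; BeginPlay binds OnShotHit to a spawn chain, and also flows straight into that chain once.
; The chain spawns a scaled-down FS_MasterField at the impact point, offset slightly against the surface normal.
; It then sets the field's activation type, short lifespan and radial magnitude, and fires it through CETrigger.
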(event Custom|OnShotHit_Event_0
  (params (HitResult :type Hit%20Result%20Structure%20%28by%20ref%29))
  (bind (_bblockinghit _binitialoverlap _time _distance _location _impactpoint _normal _impactnormal) (Collision|BreakHitResult HitResult))
  (bind _returnvalue (Game|SpawnActorfromClass "/Engine/EditorResources/FieldNodes/FS_MasterField.FS_MasterField_C" (Math|Transform|MakeTransform (+ (.location (Math|Conversions|ToTransform(Vector) _impactpoint)) (* _impactnormal "-5.000000,-5.000000,-5.000000")) "0, 0, 0" "0.700000,0.700000,0.700000") "Undefined" "MultiplyWithRoot" 0 0))
  (Variables|Default|SetChaos%20Impact%20Field _returnvalue)
  (Variables|/Engine/EditorResources/FieldNodes/FS_MasterField.FS_MasterField_C|SetActivationType (Variables|Default|GetChaos%20Impact%20Field) "NewEnumerator4")
  (Variables|/Engine/EditorResources/FieldNodes/FS_MasterField.FS_MasterField_C|SetFieldLifespan (Variables|Default|GetChaos%20Impact%20Field) 3.0)
  (Variables|/Engine/EditorResources/FieldNodes/FS_MasterField.FS_MasterField_C|SetRadial%20Magnitude (Variables|Default|GetChaos%20Impact%20Field) 1e+01)
  (Default|CETrigger (Variables|Default|GetChaos%20Impact%20Field)))

(event EventBeginPlay
  (EventDispatchers|AssignOnShotHit (delegate Custom|OnShotHit_Event_0))
  (bind _returnvalue (Game|SpawnActorfromClass "/Engine/EditorResources/FieldNodes/FS_MasterField.FS_MasterField_C" (Math|Transform|MakeTransform (+ (.location (Math|Conversions|ToTransform(Vector) (.ImpactPoint (Collision|BreakHitResult (stale Custom|OnShotHit_Event_0 HitResult))))) (* (.ImpactNormal (Collision|BreakHitResult (stale Custom|OnShotHit_Event_0 HitResult))) "-5.000000,-5.000000,-5.000000")) "0, 0, 0" "0.700000,0.700000,0.700000") "Undefined" "MultiplyWithRoot" 0 0))
  (Variables|Default|SetChaos%20Impact%20Field _returnvalue)
  (Variables|/Engine/EditorResources/FieldNodes/FS_MasterField.FS_MasterField_C|SetActivationType (Variables|Default|GetChaos%20Impact%20Field) "NewEnumerator4")
  (Variables|/Engine/EditorResources/FieldNodes/FS_MasterField.FS_MasterField_C|SetFieldLifespan (Variables|Default|GetChaos%20Impact%20Field) 3.0)
  (Variables|/Engine/EditorResources/FieldNodes/FS_MasterField.FS_MasterField_C|SetRadial%20Magnitude (Variables|Default|GetChaos%20Impact%20Field) 1e+01)
  (Default|CETrigger (Variables|Default|GetChaos%20Impact%20Field)))

(event Collision|EventActorBeginOverlap
  (params (OtherActor :type Actor%20Object%20Reference)))

(event EventTick
  (params (DeltaSeconds :type Float%20%28single-precision%29)))

(fn ConstructionScript)