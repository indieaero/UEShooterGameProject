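; Projectile actor that creates a short Chaos physics impact where it hits a surface.
; On Hit, it spawns an FS_MasterField pushed slightly into the surface along the inverted impact normal, sets its activation type, brief lifespan and radial magnitude, then triggers it.
; It then hides its sphere and point light and stops its audio, without destroying itself in this graph.
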(event EventBeginPlay)

(event Collision|EventActorBeginOverlap
  (params (OtherActor :type Actor%20Object%20Reference)))

(event EventTick
  (params (DeltaSeconds :type Float%20%28single-precision%29)))

(event Collision|EventHit
  (params (MyComp :type Primitive%20Component%20Object%20Reference) (Other :type Actor%20Object%20Reference) (OtherComp :type Primitive%20Component%20Object%20Reference) (bSelfMoved :type Boolean) (HitLocation :type Vector :default "0, 0, 0") (HitNormal :type Vector :default "0, 0, 0") (NormalImpulse :type Vector :default "0, 0, 0") (Hit :type Hit%20Result%20Structure%20%28by%20ref%29))
  (bind (_bblockinghit _binitialoverlap _time _distance _location _impactpoint _normal _impactnormal) (Collision|BreakHitResult Hit))
  (bind _returnvalue (Math|Conversions|ToTransform(Vector) _impactpoint))
  ;[1 1 1] Spawn Chaos Impact Field
  (bind _returnvalue_2 (Game|SpawnActorfromClass "/Engine/EditorResources/FieldNodes/FS_MasterField.FS_MasterField_C" (Math|Transform|MakeTransform (+ (.location _returnvalue) (* _impactnormal "-5.000000,-5.000000,-5.000000")) (.rotation _returnvalue) "0.700000,0.700000,0.700000") "Undefined" "MultiplyWithRoot" 0 0))
  (Variables|Default|SetChaosImpactFieldRef _returnvalue_2)
  (Variables|/Engine/EditorResources/FieldNodes/FS_MasterField.FS_MasterField_C|SetActivationType (Variables|Default|GetChaosImpactFieldRef) "NewEnumerator4")
  (Variables|/Engine/EditorResources/FieldNodes/FS_MasterField.FS_MasterField_C|SetFieldLifespan (Variables|Default|GetChaosImpactFieldRef) 0.1)
  (Variables|/Engine/EditorResources/FieldNodes/FS_MasterField.FS_MasterField_C|SetRadial%20Magnitude (Variables|Default|GetChaosImpactFieldRef) 1.5e+02)
  (Default|CETrigger (Variables|Default|GetChaosImpactFieldRef))
  (Rendering|SetVisibility (Variables|Default|GetPointLight) false false)
  (Audio|Components|Audio|Stop (Variables|Default|GetAudio)))

(fn ConstructionScript)