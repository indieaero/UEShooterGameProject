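; Player character Blueprint that adds zoom post-processing, running camera effects and a networked kick attack.
; While running, Tick offsets the camera and plays a camera shake; zoom state toggles the post-process blend.
; The kick notify applies radial damage at the foot socket through server authority, then multicasts a delayed impulse to nearby characters already simulating physics.
; An alternative alive-to-dead kick check remains unconnected.
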(event Custom|KickHit_Notify
  ;[1 1 1] Kick
  (if (Pawn|IsLocallyControlled)
    (if (Ability|HasAuthority)
      (CallFunction|ApplyKickRadialDamageLocal)
      (else
        (CallFunction|ServerApplyKickRadialDamage)))))

(event Custom|Server_ApplyKickRadialDamage
  ;[1 1 1] Kick
  (CallFunction|ApplyKickRadialDamageLocal))

(event Custom|Multicast_Kick
  (params (Vector :type Vector))
  ;[1 1 1] Kick
  (Utilities|FlowControl|Delay 0.1)
  (Physics|AddImpulse (Variables|Character|GetMesh) Vector "None" true))

(event EventBeginPlay)

(event Collision|EventActorBeginOverlap
  (params (OtherActor :type Actor%20Object%20Reference)))

(event EventTick
  (params (DeltaSeconds :type Float%20%28single-precision%29))
  (bind _cameracomponent (Variables|Default|GetCameraComponent))
  ;[1 1 1] Run Camera Shake
  (if (Class|STUBaseCharacter|IsRunning)
    (Transformation|SetRelativeLocation _cameracomponent "-20.000000,30.000000,-80.000000" true false)
    (Camera|PlayWorldCameraShake "/Game/VFX/Camera/BP_RunningCameraShake.BP_RunningCameraShake_C" (Transformation|GetWorldLocation _cameracomponent) 0.0 5e+02)
    (else
      (Transformation|SetRelativeLocation _cameracomponent "0, 0, 0" false false))))

(event EventOnZoomStateChanged
  (params (bIsZooming :type Boolean))
  (bind _zoompostprocess (Variables|Default|GetZoomPostProcess))
  ;[1 1 1] Zoom PostProcess
  (if bIsZooming
    (Variables|/Script/Engine.PostProcessComponent|SetBlendWeight _zoompostprocess 1.0)
    (else
      (Variables|/Script/Engine.PostProcessComponent|SetBlendWeight _zoompostprocess 0.0))))

(fn ConstructionScript)

(fn ApplyKickRadialDamageLocal
  (bind _self self)
  ;[1 1 1] Logic Kick
  (LocalVariables|SetKickOrigin (Transformation|GetSocketLocation (Variables|Character|GetMesh) "KickImpact"))
  (LocalVariables|SetKickRadius 1e+02)
  (Game|Damage|ApplyRadialDamage 5e+01 (+ (LocalVariables|GetKickOrigin) "15.000000,0.000000,0.000000") (LocalVariables|GetKickRadius) "/Script/Engine.DamageType" (Utilities|Array|MakeArray _self) _self (Pawn|GetController) true "ECC_Visibility")
  (Camera|PlayWorldCameraShake "/Game/VFX/Camera/BP_DamageCameraShake.BP_DamageCameraShake_C" (Transformation|GetWorldLocation (Variables|Default|GetCameraComponent)) 0.0 5e+02)
  (bind _outactors (Collision|SphereOverlapActors (LocalVariables|GetKickOrigin) (LocalVariables|GetKickRadius) (Utilities|Array|MakeArray "ObjectTypeQuery3") "BP_STUPlayerCharacter_C" (Utilities|Array|MakeArray self)))
  (for _array_element _outactors
    (bind _asbp_stuplayer_character (Utilities|Casting|CastToBP_STUPlayerCharacter _array_element))
    (if (Physics|IsSimulatingPhysics (Variables|/Script/Engine.Character|GetMesh _asbp_stuplayer_character) "None")
      (CallFunction|MulticastKick _asbp_stuplayer_character (+ (* (Transformation|GetActorForwardVector) (LocalVariables|GetKickPower)) (Math|Vector|MakeVector 0.0 0.0 (LocalVariables|GetUpPower))))))
  (return))